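; FloorRespawning is a floor actor that chains copies of itself ahead of the runner character to extend the track.
; BeginPlay caches the player as BP_RunnerCharacter, and both overlap events respond only to that character.
; Overlapping the Create component spawns a new FloorRespawning at the Arrow component's world transform.
; Overlapping the Delete component destroys the current floor, with no pooling.
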(event OnComponentBeginOverlap(create)
  (params (OverlappedComponent :type Primitive%20Component%20Object%20Reference) (OtherActor :type Actor%20Object%20Reference) (OtherComp :type Primitive%20Component%20Object%20Reference) (OtherBodyIndex :type Integer) (bFromSweep :type Boolean) (SweepResult :type Hit%20Result%20Structure%20%28by%20ref%29))
  (if (== OtherActor (Variables|Default|GetAs%20BP%20Runner%20Character))
    (Game|SpawnActorfromClass "FloorRespawning_C" (Transformation|GetWorldTransform (Variables|Default|GetArrow)) "Undefined" "MultiplyWithRoot" 0 (Game|GetPlayerCharacter 0))))

(event OnComponentBeginOverlap(delete)
  (params (OverlappedComponent :type Primitive%20Component%20Object%20Reference) (OtherActor :type Actor%20Object%20Reference) (OtherComp :type Primitive%20Component%20Object%20Reference) (OtherBodyIndex :type Integer) (bFromSweep :type Boolean) (SweepResult :type Hit%20Result%20Structure%20%28by%20ref%29))
  (if (== OtherActor (Variables|Default|GetAs%20BP%20Runner%20Character))
    (Actor|DestroyActor)))

(event EventBeginPlay
  (bind _asbp_runner_character (Utilities|Casting|CastToBP_RunnerCharacter (Game|GetPlayerCharacter 0)))
  (Variables|Default|SetAs%20BP%20Runner%20Character _asbp_runner_character))

(fn ConstructionScript)